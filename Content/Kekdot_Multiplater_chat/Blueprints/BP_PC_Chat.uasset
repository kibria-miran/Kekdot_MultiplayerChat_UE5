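; BP_PC_Chat is a player controller that handles multiplayer text chat.
; On BeginPlay the local controller creates and displays a WB_ChatPanel, and Enter focuses its input box.
; SR_SubmitChat, named as a server event, loops through the GameState PlayerArray and relays the name and message to each player's controller.
; Each controller's OC_UpdateChat, named as an owning-client event, passes them to its chat panel.
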(event Custom|SR_SubmitChat
  (params (Player%20Name :type Text) (Chat%20Message :type Text))
  (for _array_element (Variables|/Script/Engine.GameStateBase|GetPlayerArray (Game|GetGameState))
    (bind _asbp_pc_chat (Utilities|Casting|CastToBP_PC_Chat (Game|GetPlayerController _array_element)))
    (CallFunction|OCUpdateChat _asbp_pc_chat Player%20Name Chat%20Message)))

(event Custom|OC_UpdateChat
  (params (Player%20Name :type Text) (Chat%20Message :type Text))
  (bind _wb_chatpanel (Variables|Default|GetWB_ChatPanel)
    (:then
      (Default|UpdateChat _wb_chatpanel Player%20Name Chat%20Message))
    (:else)))

(event EventBeginPlay
  (if (Pawn|IsLocalPlayerController)
    (bind _returnvalue (UserInterface|CreateWidget "/Game/Kekdot_Multiplater_chat/Widgets/WB_ChatPanel.WB_ChatPanel_C" self))
    (bind _output_get (Variables|Default|SetWB_ChatPanel _returnvalue))
    (UserInterface|Viewport|AddtoViewport _output_get 0)))

(event Input|KeyboardEvents|Enter
  (params (Key :type Key%20Structure :default "None"))
  (:Pressed
    (bind _wb_chatpanel (Variables|Default|GetWB_ChatPanel)
      (:then
        (Widget|SetFocus (Variables|/Game/Kekdot_Multiplater_chat/Widgets/WB_ChatPanel.WB_ChatPanel_C|GetChatInputBox _wb_chatpanel)))
      (:else))))

(fn ConstructionScript)